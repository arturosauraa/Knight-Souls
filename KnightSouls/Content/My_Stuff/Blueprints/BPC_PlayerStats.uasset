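; Player stats component for BP_ThirdPersonCharacter that tracks health, stamina, XP and level.
; On BeginPlay it waits a tick, caches the character, then initializes its HUD, which each change function updates directly.
; Decrease functions return true on depletion; XP overflow carries into the next level, which raises MaxXP.
; The over-max checks in IncreaseHealth and IncreaseStamina assign max to itself, so current values are never clamped.
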(event EventBeginPlay
  (Utilities|FlowControl|DelayUntilNextTick)
  (bind _asbp_third_person_character (Utilities|Casting|CastToBP_ThirdPersonCharacter (Components|GetOwner)))
  (Variables|Default|SetPlayer%20BP _asbp_third_person_character)
  (Progress|SetPercent (Variables|/Game/My_Stuff/UI/WB_HUD.WB_HUD_C|GetStaminaBar (Variables|/Game/ThirdPerson/Blueprints/BP_ThirdPersonCharacter.BP_ThirdPersonCharacter_C|GetHUD%20Widget (Variables|Default|GetPlayer%20BP))) (/ (Variables|Stamina|GetCurrent%20Stamina) (Variables|Stamina|GetMax%20Stamina)))
  (Progress|SetPercent (Variables|/Game/My_Stuff/UI/WB_HUD.WB_HUD_C|GetHealthBar (Variables|/Game/ThirdPerson/Blueprints/BP_ThirdPersonCharacter.BP_ThirdPersonCharacter_C|GetHUD%20Widget (Variables|Default|GetPlayer%20BP))) (/ (Variables|Health|GetCurrent%20Health) (Variables|Health|GetMax%20Health)))
  (Progress|SetPercent (Variables|/Game/My_Stuff/UI/WB_HUD.WB_HUD_C|GetXPBar (Variables|/Game/ThirdPerson/Blueprints/BP_ThirdPersonCharacter.BP_ThirdPersonCharacter_C|GetHUD%20Widget (Variables|Default|GetPlayer%20BP))) (/ (Variables|XPLevel|GetXP) (Variables|XPLevel|GetMax%20XP)))
  (Rendering|Components|TextRender|SetText (Variables|/Game/My_Stuff/UI/WB_HUD.WB_HUD_C|GetLevelText (Variables|/Game/ThirdPerson/Blueprints/BP_ThirdPersonCharacter.BP_ThirdPersonCharacter_C|GetHUD%20Widget (Variables|Default|GetPlayer%20BP))) (Utilities|Text|ToText(Integer) (Variables|XPLevel|GetLevel))))

(event EventTick
  (params (DeltaSeconds :type Float%20%28single-precision%29)))

(fn DecreaseHealth
  (params (Damage :type Float%20%28double-precision%29))
  (if (not (<= (Variables|Health|GetCurrent%20Health) 0.0))
    (bind _output_get (Variables|Health|SetCurrent%20Health (- (Variables|Health|GetCurrent%20Health) Damage)))
    (Progress|SetPercent (Variables|/Game/My_Stuff/UI/WB_HUD.WB_HUD_C|GetHealthBar (Variables|/Game/ThirdPerson/Blueprints/BP_ThirdPersonCharacter.BP_ThirdPersonCharacter_C|GetHUD%20Widget (Variables|Default|GetPlayer%20BP))) (/ _output_get (Variables|Health|GetMax%20Health)))
    (if (<= (Variables|Health|GetCurrent%20Health) 0.0)
      _
      (else
        (return false))))
  (return true))

(fn IncreaseMaxHealth
  (params (Health%20Increase :type Float%20%28double-precision%29))
  (Variables|Health|SetMax%20Health (+ (Variables|Health|GetMax%20Health) Health%20Increase))
  (Progress|SetPercent (Variables|/Game/My_Stuff/UI/WB_HUD.WB_HUD_C|GetHealthBar (Variables|/Game/ThirdPerson/Blueprints/BP_ThirdPersonCharacter.BP_ThirdPersonCharacter_C|GetHUD%20Widget (Variables|Default|GetPlayer%20BP))) (/ (Variables|Health|GetCurrent%20Health) (Variables|Health|GetMax%20Health))))

(fn DecreaseStamina
  (params (Drain%20Stamina :type Float%20%28double-precision%29))
  (if (not (<= (Variables|Stamina|GetCurrent%20Stamina) 0.0))
    (Variables|Stamina|SetCurrent%20Stamina (- (Variables|Stamina|GetCurrent%20Stamina) Drain%20Stamina))
    (Progress|SetPercent (Variables|/Game/My_Stuff/UI/WB_HUD.WB_HUD_C|GetStaminaBar (Variables|/Game/ThirdPerson/Blueprints/BP_ThirdPersonCharacter.BP_ThirdPersonCharacter_C|GetHUD%20Widget (Variables|Default|GetPlayer%20BP))) (/ (Variables|Stamina|GetCurrent%20Stamina) (Variables|Stamina|GetMax%20Stamina)))
    (if (<= (Variables|Stamina|GetCurrent%20Stamina) 0.0)
      _
      (else
        (return false))))
  (return true))

(fn IncreaseMaxStamina
  (params (Added%20Stamina :type Float%20%28double-precision%29))
  (Variables|Stamina|SetMax%20Stamina (+ (Variables|Stamina|GetMax%20Stamina) Added%20Stamina))
  (Progress|SetPercent (Variables|/Game/My_Stuff/UI/WB_HUD.WB_HUD_C|GetStaminaBar (Variables|/Game/ThirdPerson/Blueprints/BP_ThirdPersonCharacter.BP_ThirdPersonCharacter_C|GetHUD%20Widget (Variables|Default|GetPlayer%20BP))) (/ (Variables|Stamina|GetCurrent%20Stamina) (Variables|Stamina|GetMax%20Stamina))))

(fn IncreaseHealth
  (params (Add%20Health :type Float%20%28double-precision%29))
  (Variables|Health|SetCurrent%20Health (+ (Variables|Health|GetCurrent%20Health) Add%20Health))
  (if (> (Variables|Health|GetCurrent%20Health) (Variables|Health|GetMax%20Health))
    (Variables|Health|SetMax%20Health (Variables|Health|GetMax%20Health)))
  (Progress|SetPercent (Variables|/Game/My_Stuff/UI/WB_HUD.WB_HUD_C|GetHealthBar (Variables|/Game/ThirdPerson/Blueprints/BP_ThirdPersonCharacter.BP_ThirdPersonCharacter_C|GetHUD%20Widget (Variables|Default|GetPlayer%20BP))) (/ (Variables|Health|GetCurrent%20Health) (Variables|Health|GetMax%20Health))))

(fn IncreaseStamina
  (params (Add%20Stamina :type Float%20%28double-precision%29))
  (Variables|Stamina|SetCurrent%20Stamina (+ (Variables|Stamina|GetCurrent%20Stamina) Add%20Stamina))
  (if (> (Variables|Stamina|GetCurrent%20Stamina) (Variables|Stamina|GetMax%20Stamina))
    (Variables|Stamina|SetMax%20Stamina (Variables|Stamina|GetMax%20Stamina)))
  (Progress|SetPercent (Variables|/Game/My_Stuff/UI/WB_HUD.WB_HUD_C|GetStaminaBar (Variables|/Game/ThirdPerson/Blueprints/BP_ThirdPersonCharacter.BP_ThirdPersonCharacter_C|GetHUD%20Widget (Variables|Default|GetPlayer%20BP))) (/ (Variables|Stamina|GetCurrent%20Stamina) (Variables|Stamina|GetMax%20Stamina))))

(fn IncreaseXP
  (params (Added%20XP :type Float%20%28double-precision%29))
  (Variables|XPLevel|SetXP (+ (Variables|XPLevel|GetXP) Added%20XP))
  (if (>= (Variables|XPLevel|GetXP) (Variables|XPLevel|GetMax%20XP))
    (Variables|XPLevel|SetXP%20Left (- (Variables|XPLevel|GetXP) (Variables|XPLevel|GetMax%20XP)))
    (XPLevel|IncreaseLevel 1))
  (Progress|SetPercent (Variables|/Game/My_Stuff/UI/WB_HUD.WB_HUD_C|GetXPBar (Variables|/Game/ThirdPerson/Blueprints/BP_ThirdPersonCharacter.BP_ThirdPersonCharacter_C|GetHUD%20Widget (Variables|Default|GetPlayer%20BP))) (/ (Variables|XPLevel|GetXP) (Variables|XPLevel|GetMax%20XP))))

(fn IncreaseLevel
  (params (Added%20Level :type Integer))
  (Variables|XPLevel|SetLevel (+ (Variables|XPLevel|GetLevel) Added%20Level))
  (Variables|XPLevel|SetMax%20XP (+ (Variables|XPLevel|GetMax%20XP) 1e+02))
  (Variables|XPLevel|SetXP (Variables|XPLevel|GetXP%20Left))
  (Rendering|Components|TextRender|SetText (Variables|/Game/My_Stuff/UI/WB_HUD.WB_HUD_C|GetLevelText (Variables|/Game/ThirdPerson/Blueprints/BP_ThirdPersonCharacter.BP_ThirdPersonCharacter_C|GetHUD%20Widget (Variables|Default|GetPlayer%20BP))) (Utilities|Text|ToText(Integer) (Variables|XPLevel|GetLevel))))