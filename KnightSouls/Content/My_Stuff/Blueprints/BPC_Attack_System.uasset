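; Attack component for BP_ThirdPersonCharacter that runs a three-hit melee sword combo (right slash, left slash, stab) from IA_Attack.
; Clicks during an attack are buffered in SaveAttack, and AttackCombo either plays the next montage by AttackIndex or resets the combo.
; A looping timer sphere-traces along the blade between start and stop events, while StabTrace does a one-shot check.
; Hits on "Damageable" actors apply damage, camera shake, sound and blood.
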(event Custom|Attack%20Start
  ;[1 1 1] Attack System
  ;;[1 1 1] Attack
  (if (Variables|Default|Getis%20Attacking?)
    (Variables|Default|Setsave%20Attack? true)
    (else
      (Variables|Default|Setis%20Attacking? true)
      (switch int (Variables|Default|GetAttack%20Index)
        (:0
          (CallFunction|SwordAttack1))
        (:1
          (CallFunction|SwordAttack2))
        (:2
          (CallFunction|SwordAttack3))))))

(event Custom|Attack%20Combo
  ;[1 1 1] Attack System
  ;;[1 1 1] Combo Continue
  (if (Variables|Default|Getsave%20Attack?)
    (Variables|Default|Setsave%20Attack? false)
    (switch int (Variables|Default|GetAttack%20Index)
      (:0
        (CallFunction|SwordAttack1))
      (:1
        (CallFunction|SwordAttack2))
      (:2
        (CallFunction|SwordAttack3)))
    (else
      (CallFunction|StopCombo))))

(event Custom|Play%20Sword%20Hit%20Sound
  (bind _returnvalue (Components|GetOwner))
  (bind _returnvalue_2 (Transformation|GetActorLocation _returnvalue))
  ;[1 1 1] Play Sword hit Sounds
  (Audio|PlaySoundatLocation "/Game/My_Stuff/Audio/Damage/Hit.Hit" _returnvalue_2 "0, 0, 0" 0.5 1.0 0.0 "/Game/My_Stuff/Audio/SA_Character.SA_Character" 0 0 0)
  (Audio|PlaySoundatLocation "/Game/My_Stuff/Audio/Damage/Sword_Hit.Sword_Hit" _returnvalue_2 "0, 0, 0" 0.5 1.0 0.0 "/Game/My_Stuff/Audio/SA_Character.SA_Character" 0 0 0))

(event Custom|Stop%20Combo
  ;[1 1 1] Attack System
  ;;[1 1 1] Stop Combo/Attack
  (Variables|Default|Setis%20Attacking? false)
  (Variables|Default|SetAttack%20Index 0))

(event Custom|Sword%20Attack%203
  ;[1 1 1] Attack System
  ;;[1 1 1] Sword Attack 3
  (Utilities|FlowControl|DoOnce false :!label _label
    (:Completed
      (Utilities|FlowControl|Delay 0.1)
      (Animation|Montage|PlayMontage (Variables|Default|GetMesh) "/Game/My_Stuff/Character/Animations/Sword_Attacks/Stabbing_Montage.Stabbing_Montage" 1.5
        (:then
          (Variables|Default|SetAttack%20Index 3)
          (goto _label Reset))))))

(event Custom|Sword%20Attack%201
  ;[1 1 1] Attack System
  ;;[1 1 1] Sword Attack 1
  (Utilities|FlowControl|DoOnce false :!label _label
    (:Completed
      (Utilities|FlowControl|Delay 0.1)
      (Animation|Montage|PlayMontage (Variables|Default|GetMesh) "/Game/My_Stuff/Character/Animations/Sword_Attacks/Right_Slashing_Montage.Right_Slashing_Montage" 1.5
        (:then
          (Variables|Default|SetAttack%20Index 1)
          (goto _label Reset))))))

(event Custom|Start%20Sword%20Trace
  ;[1 1 1] Sword Trace
  (bind _returnvalue (Utilities|Time|SetTimerbyEvent (delegate Custom|Sword%20Trace%20Loop) 0.01 true))
  (Variables|Default|SetSwordTraceLoop _returnvalue))

(event Custom|Sword%20Attack%202
  ;[1 1 1] Attack System
  ;;[1 1 1] Sword Attack 2
  (Utilities|FlowControl|DoOnce false :!label _label
    (:Completed
      (Utilities|FlowControl|Delay 0.1)
      (Animation|Montage|PlayMontage (Variables|Default|GetMesh) "/Game/My_Stuff/Character/Animations/Sword_Attacks/Left_Slash_Montage.Left_Slash_Montage" 1.5
        (:then
          (Variables|Default|SetAttack%20Index 2)
          (goto _label Reset))))))

(event Custom|Sword%20Trace%20Loop
  ;[1 1 1] Sword Trace
  (bind (_outhit _returnvalue) (Collision|SphereTraceByChannel (Transformation|GetWorldLocation (Variables|/Game/ThirdPerson/Blueprints/BP_ThirdPersonCharacter.BP_ThirdPersonCharacter_C|GetSwordBottom (Variables|Default|GetCharacter%20BP))) (Transformation|GetWorldLocation (Variables|/Game/ThirdPerson/Blueprints/BP_ThirdPersonCharacter.BP_ThirdPersonCharacter_C|GetSwordTop (Variables|Default|GetCharacter%20BP))) 12.0 "TraceTypeQuery1" false 0 "None" true "(R=1.000000,G=0.000000,B=0.000000,A=1.000000)" "(R=0.000000,G=1.000000,B=0.000000,A=1.000000)" 0.1))
  (if _returnvalue
    (if (Actor|ActorHasTag (.HitActor (Collision|BreakHitResult _outhit)) "Damageable")
      (Utilities|FlowControl|DoOnce false :!label _label
        (:Completed
          (Game|Damage|ApplyDamage (.HitActor (Collision|BreakHitResult _outhit)) 1e+01 0 0)
          (Camera|PlayWorldCameraShake "/Game/My_Stuff/Blueprints/BP_Sword_Hit_CameraShake.BP_Sword_Hit_CameraShake_C" (.Location (Collision|BreakHitResult _outhit)) 0.0 2e+03)
          (CallFunction|PlaySwordHitSound)
          (Effects|SpawnEmitteratLocation "/Game/FX/Particles/Blood/P_Blood_Splat_Cone.P_Blood_Splat_Cone" (.Location (Collision|BreakHitResult _outhit)) (Math|Rotator|MakeRotfromXY (.Normal (Collision|BreakHitResult _outhit)) (.Normal (Collision|BreakHitResult _outhit))) "0.400000,0.400000,0.400000" true "AutoRelease")
          (Utilities|FlowControl|Delay 0.5)
          (goto _label Reset))))))

(event Custom|StopSwordTrace
  ;[1 1 1] Sword Trace
  (Utilities|Time|ClearandInvalidateTimerbyHandle (Variables|Default|GetSwordTraceLoop)))

(event Custom|Stab%20Trace
  (bind _character_bp (Variables|Default|GetCharacter%20BP))
  (bind _stabtrace (Variables|/Game/ThirdPerson/Blueprints/BP_ThirdPersonCharacter.BP_ThirdPersonCharacter_C|GetStabTrace _character_bp))
  (bind _returnvalue (Transformation|GetWorldLocation _stabtrace))
  ;[1 1 1] Stab Trace (Stab and Kick)
  (bind (_outhit _returnvalue_2) (Collision|SphereTraceByChannel _returnvalue _returnvalue 25.0 "TraceTypeQuery1" false 0 "None" true "(R=1.000000,G=0.000000,B=0.000000,A=1.000000)" "(R=0.000000,G=1.000000,B=0.000000,A=1.000000)" 0.5))
  (if _returnvalue_2
    (if (Actor|ActorHasTag (.HitActor (Collision|BreakHitResult _outhit)) "Damageable")
      (Game|Damage|ApplyDamage (.HitActor (Collision|BreakHitResult _outhit)) 1e+01 0 0)
      (Utilities|FlowControl|Delay 0.5)
      (Camera|PlayWorldCameraShake "/Game/My_Stuff/Blueprints/BP_Sword_Hit_CameraShake.BP_Sword_Hit_CameraShake_C" (.Location (Collision|BreakHitResult _outhit)) 0.0 2e+03)
      (CallFunction|PlaySwordHitSound)
      (Effects|SpawnEmitteratLocation "/Game/FX/Particles/Blood/P_Blood_Splat_Cone.P_Blood_Splat_Cone" (.Location (Collision|BreakHitResult _outhit)) (Math|Rotator|MakeRotfromXY (.Normal (Collision|BreakHitResult _outhit)) (.Normal (Collision|BreakHitResult _outhit))) "0.400000,0.400000,0.400000" true "AutoRelease"))))

(event Input|EnhancedActionEvents|EnhancedInputActionIA_Attack
  (params (ActionValue :type Boolean) (ElapsedSeconds :type Float%20%28double-precision%29) (TriggeredSeconds :type Float%20%28double-precision%29) (InputAction :type Input%20Action%20Object%20Reference :default "/Game/ThirdPerson/Input/Actions/IA_Attack.IA_Attack"))
  ;[1 1 1] Attack System
  ;;[1 1 1] Attack On Click
  (:Started
    (if (Variables|Default|Getcan%20Attack?)
      (CallFunction|AttackStart))))

(event EventBeginPlay
  (bind _asbp_third_person_character (Utilities|Casting|CastToBP_ThirdPersonCharacter (Components|GetOwner)))
  (Variables|Default|SetCharacter%20BP _asbp_third_person_character)
  (Variables|Default|SetMesh (Variables|/Script/Engine.Character|GetMesh _asbp_third_person_character)))